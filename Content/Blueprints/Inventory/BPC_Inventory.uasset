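; Inventory component that creates the WB_Inventory widget on BeginPlay and holds an item array sized to the widget's slot count.
; AddToInventory walks the array in order, filling the first empty entry or adding quantity to a same-named one, whichever comes first, and returns false when neither exists.
; Each successful add calls RefreshInventory, which redraws every slot's icon from the first flipbook frame and its quantity text.
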(event `self.ReceiveBeginPlay`
  (bind _returnvalue (`|CreateWidget` "/Game/Blueprints/Inventory/WB_Inventory.WB_Inventory_C" (`GameplayStatics.GetPlayerController` 0)))
  (set `self.Inventory` _returnvalue)
  (`self.InitializeInventory`)
  (`self.RefreshInventory`)
  (`UserWidget.AddToViewport` (`self.Inventory`) 0))

(fn `AddToInventory`
  (params (ItemToAdd :type "/Game/Items/S_Item Structure"))
  (returns (ItemAdded :type Boolean))
  (locals (Item :type "/Game/Items/S_Item Structure") (CurrentItem :type "/Game/Items/S_Item Structure") (CurrentIndex :type Integer))
  (set `local.Item` ItemToAdd)
  (for (_array_element _array_index) (`self.Items`)
    (set `local.CurrentItem` _array_element)
    (set `local.CurrentIndex` _array_index)
    (if (`KismetStringLibrary.IsEmpty` (`.Name_2_F105B8C74B0571DA9CAC8E9F97E08A39` (break `/Game/Items/S_Item` (`local.CurrentItem`))))
      (`KismetArrayLibrary.Array_Set` (`self.Items`) (`local.CurrentIndex`) (`local.Item`))
      (`self.RefreshInventory`)
      (return true)
      (elif (`KismetStringLibrary.EqualEqual_StrStr` (`.Name_2_F105B8C74B0571DA9CAC8E9F97E08A39` (break `/Game/Items/S_Item` (`local.CurrentItem`))) (`.Name_2_F105B8C74B0571DA9CAC8E9F97E08A39` (break `/Game/Items/S_Item` (`local.Item`))))
        (bind _structout (setmembers `/Game/Items/S_Item` :`StructRef` (`local.CurrentItem`) :`Quantity` (+ (`.Quantity_14_D3DE4E164A4FA8C0E1E0ACA55132B535` (break `/Game/Items/S_Item` (`local.CurrentItem`))) (`.Quantity_14_D3DE4E164A4FA8C0E1E0ACA55132B535` (break `/Game/Items/S_Item` (`local.Item`))))))
        (`KismetArrayLibrary.Array_Set` (`self.Items`) (`local.CurrentIndex`) _structout)
        (`self.RefreshInventory`)
        (return true))))
  (return false))

(fn `InitializeInventory`
  (for _ (`PanelWidget.GetAllChildren` (`/Game/Blueprints/Inventory/WB_Inventory.Slots` (`self.Inventory`)))
    (`KismetArrayLibrary.Array_Add` (`self.Items`) (make `/Game/Items/S_Item` "" null null))))

(fn `RefreshInventory`
  (locals (Slot :type "/Game/Blueprints/Inventory/WB_InventorySlot Object Reference"))
  (for (_array_element _array_index) (`self.Items`)
    (bind _aswb_inventory_slot (cast `/Game/Blueprints/Inventory/WB_InventorySlot` (`PanelWidget.GetChildAt` (`/Game/Blueprints/Inventory/WB_Inventory.Slots` (`self.Inventory`)) _array_index)))
    (set `local.Slot` _aswb_inventory_slot)
    (if (`KismetStringLibrary.IsEmpty` (break `/Game/Items/S_Item` _array_element))
      (`Image.SetBrush` (`/Game/Blueprints/Inventory/WB_InventorySlot.Item` (`local.Slot`)) (`WidgetBlueprintLibrary.MakeBrushFromMaterial` null))
      (else
        (`Image.SetBrush` (`/Game/Blueprints/Inventory/WB_InventorySlot.Item` (`local.Slot`)) (`PaperSpriteBlueprintLibrary.MakeBrushFromSprite` (`PaperFlipbook.GetSpriteAtFrame` (`.FlipBook_8_CEB189B145ED1EC8F4FF8AB46C18548B` (break `/Game/Items/S_Item` _array_element)) 0)))))
    (if (== (`.Quantity_14_D3DE4E164A4FA8C0E1E0ACA55132B535` (break `/Game/Items/S_Item` _array_element)) 0)
      (set `TextBlock.Text` "" (`/Game/Blueprints/Inventory/WB_InventorySlot.Quantity` (`local.Slot`)))
      (else
        (set `TextBlock.Text` (`KismetTextLibrary.Conv_IntToText` (`.Quantity_14_D3DE4E164A4FA8C0E1E0ACA55132B535` (break `/Game/Items/S_Item` _array_element))) (`/Game/Blueprints/Inventory/WB_InventorySlot.Quantity` (`local.Slot`)))))))