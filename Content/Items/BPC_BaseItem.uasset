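; Base item Blueprint that shows a Paper2D flipbook taken from its Item data and responds to player pointing and interaction.
; On BeginPlay it applies the item's flipbook, while the pointed-at and not-pointed-at events only print the item's name.
; Interact constructs an object from the item's action class and sends it an interact message with player character 0 and itself, delegating behavior to that class.
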(event `self.ReceiveBeginPlay`
  (bind (_item_name _item_flipbook) (break `/Game/Items/S_Item` (`self.Item`)))
  (`PaperFlipbookComponent.SetFlipbook` (`self.PaperFlipbook`) _item_flipbook))

(event `/Game/Items/I_Interact.PointedAt`
  (bind _item_name (break `/Game/Items/S_Item` (`self.Item`)))
  (`KismetSystemLibrary.PrintString` (`KismetStringLibrary.Concat_StrStr` "Pointed At " _item_name)))

(event `/Game/Items/I_Interact.NotPointedAt`
  (bind _item_name (break `/Game/Items/S_Item` (`self.Item`)))
  (`KismetSystemLibrary.PrintString` (`KismetStringLibrary.Concat_StrStr` "Not pointed At " _item_name)))

(event `/Game/Items/I_Interact.Interact`
  (bind (_item_name _item_flipbook _item_interractaction) (break `/Game/Items/S_Item` (`self.Item`)))
  (bind _returnvalue (`|GenericCreateObject` _item_interractaction))
  (message `/Game/Items/ItemActions/I_ItemAction.Interract` _returnvalue (`GameplayStatics.GetPlayerCharacter` 0) self))

(fn `UserConstructionScript`)